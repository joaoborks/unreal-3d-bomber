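; BP_BombRemote is a remote bomb that calls Detonate when its RemoteActivated event fires.
; The construction script creates a dynamic instance of M_Bomb on the Sphere and sets a dark blue base color with a white glow.
; On BeginPlay, a timeline drives the material's emissive intensity to animate the glow.
; The detonation logic itself is defined outside these graphs.
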(event Custom|RemoteActivated
  (Class|Bomb|Detonate))

(event EventBeginPlay
  (bind _emissivevalue (Timeline|RemoteBombGlowTimeline PlayFromStart)
    (:Update
      (Rendering|Material|SetScalarParameterValue (Variables|Default|GetDynamicMaterial) "EmissiveIntensity" _emissivevalue :!class /Script/Engine.MaterialInstanceDynamic))))

(fn ConstructionScript
  (bind _returnvalue (Rendering|Material|CreateDynamicMaterialInstance (Variables|Default|GetSphere) 0 "/Game/_Project/Materials/M_Bomb.M_Bomb" :!class /Script/Engine.PrimitiveComponent))
  (bind _output_get (Variables|Default|SetDynamicMaterial _returnvalue))
  (Rendering|Material|SetVectorParameterValue _output_get "BaseColor" "(R=0.055429,G=0.047461,B=0.270833,A=1.000000)" :!class /Script/Engine.MaterialInstanceDynamic)
  (Rendering|Material|SetVectorParameterValue _output_get "GlowColor" "(R=1.000000,G=1.000000,B=1.000000,A=1.000000)" :!class /Script/Engine.MaterialInstanceDynamic))