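; BP_PlayerChar is the player character in a Bomberman-style game.
; A bomb blast hit reports the player's death to the game mode.
; A remote bomb pickup event swaps the bomb class to the remote variant, then reverts to the standard bomb after a retriggerable delay, so repeat calls restart the timer.
; The construction script tints the mesh through a dynamic material and sets the default bomb class.
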(event Custom|GetRemoteBomb
  (Variables|Default|SetHasRemote true)
  (Variables|Default|SetBombBP "/Game/_Project/Blueprints/Dynamic/BP_BombRemote.BP_BombRemote_C")
  (Utilities|FlowControl|RetriggerableDelay (Variables|PlayerChar|GetRemoteBombDuration))
  (Variables|Default|SetHasRemote false)
  (Variables|Default|SetBombBP "/Game/_Project/Blueprints/Dynamic/BP_Bomb.BP_Bomb_C"))

(event EventOnBombBlastHit
  (bind _asbp_unreal_bomberman_game_mode (Utilities|Casting|CastToBP_UnrealBombermanGameMode (Game|GetGameMode)))
  (Default|PlayerDeath _asbp_unreal_bomberman_game_mode self))

(fn ConstructionScript
  (bind _returnvalue (Rendering|Material|CreateDynamicMaterialInstance (Variables|Default|GetStaticMesh) 0 "/Game/_Project/Materials/M_FlatMaterial.M_FlatMaterial" :!class /Script/Engine.PrimitiveComponent))
  (bind _output_get (Variables|Default|SetDynamicMaterial _returnvalue))
  (Rendering|Material|SetVectorParameterValue _output_get "Color" "(R=0.118139,G=0.340270,B=0.609375,A=1.000000)" :!class /Script/Engine.MaterialInstanceDynamic)
  (Variables|Default|SetBombBP "/Game/_Project/Blueprints/Dynamic/BP_Bomb.BP_Bomb_C"))