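; BP_Powerup is a pickup that grants the player character a speed boost, an extra bomb, longer blast range or a remote bomb.
; The construction script picks a random pickup type and sets the matching billboard icon.
; When an actor of exactly the BP_PlayerChar class overlaps the box, the pickup applies that type's effect directly to the player, then destroys itself.
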(event OnComponentBeginOverlap(Box)
  (params (OverlappedComponent :type Primitive%20Component%20Object%20Reference) (OtherActor :type Actor%20Object%20Reference) (OtherComp :type Primitive%20Component%20Object%20Reference) (OtherBodyIndex :type Integer) (bFromSweep :type Boolean) (SweepResult :type Hit%20Result%20Structure%20%28by%20ref%29))
  (Variables|Default|SetPlayerRef OtherActor)
  (if (== "/Game/_Project/Blueprints/BP_PlayerChar.BP_PlayerChar_C" (Utilities|GetClass OtherActor))
    (Utilities|FlowControl|Sequence
      (:then_0
        (bind _asbp_player_char (Utilities|Casting|CastToBP_PlayerChar (Variables|Default|GetPlayerRef)))
        (switch Utilities|FlowControl|Switch|SwitchonE_PickupTypeEnum (Variables|Default|GetPickupType)
          (:NewEnumerator0
            (Variables|/Script/Engine.CharacterMovementComponent|SetMaxWalkSpeed (Variables|/Script/Engine.Character|GetCharacterMovement _asbp_player_char) (+ (Variables|Default|GetSpeedBoost) (Variables|/Script/Engine.CharacterMovementComponent|GetMaxWalkSpeed (Variables|/Script/Engine.Character|GetCharacterMovement _asbp_player_char)))))
          (:NewEnumerator1
            (Variables|/Game/_Project/Blueprints/BP_PlayerChar.BP_PlayerChar_C|SetBombLimit _asbp_player_char (+ (Variables|/Game/_Project/Blueprints/BP_PlayerChar.BP_PlayerChar_C|GetBombLimit _asbp_player_char) 1)))
          (:NewEnumerator2
            (Variables|/Game/_Project/Blueprints/BP_PlayerChar.BP_PlayerChar_C|SetBombRange _asbp_player_char (+ (Variables|/Game/_Project/Blueprints/BP_PlayerChar.BP_PlayerChar_C|GetBombRange _asbp_player_char) 1.0)))
          (:NewEnumerator3
            (Default|GetRemoteBomb _asbp_player_char))))
      (:then_1
        (Actor|DestroyActor)))))

(fn ConstructionScript
  (bind _billboard (Variables|Default|GetBillboard))
  (bind _output_get (Variables|Default|SetPickupType (Utilities|Enum|ByteToEnumE_PickupTypeEnum (Math|Conversions|ToByte(Integer) (Math|Random|RandomIntegerinRange 0 3)))))
  (switch Utilities|FlowControl|Switch|SwitchonE_PickupTypeEnum _output_get
    (:NewEnumerator0
      (Rendering|Components|Sprite|SetSprite _billboard "/Game/_Project/Textures/SpeedIcon.SpeedIcon"))
    (:NewEnumerator1
      (Rendering|Components|Sprite|SetSprite _billboard "/Game/_Project/Textures/BombIcon.BombIcon"))
    (:NewEnumerator2
      (Rendering|Components|Sprite|SetSprite _billboard "/Game/_Project/Textures/LongerBlastsIcon.LongerBlastsIcon"))
    (:NewEnumerator3
      (Rendering|Components|Sprite|SetSprite _billboard "/Game/_Project/Textures/RemoteIcon.RemoteIcon"))))