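; BP_Bomb is a timed bomb whose sphere glows on a timeline before it detonates.
; The construction script creates a dynamic instance of M_Bomb and assigns BP_BlastFx as the blast effect.
; On BeginPlay, the glow timeline is scaled by BlastTime and drives the material's emissive intensity.
; When the timeline finishes, OnBlastTimeEnd calls Detonate, whose logic is not defined in this graph.
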(event EventBeginPlay
  (Components|Timeline|SetPlayRate (Variables|Default|GetGlowTimeline) (/ 1.0 (Variables|Bomb|GetBlastTime)))
  (bind _emissivevalue (Timeline|GlowTimeline PlayFromStart)
    (:Update
      (Rendering|Material|SetScalarParameterValue (Variables|Default|GetDynamicMaterial) "EmissiveIntensity" _emissivevalue :!class /Script/Engine.MaterialInstanceDynamic))
    (:Finished
      (CallFunction|OnBlastTimeEnd))))

(fn ConstructionScript
  (bind _returnvalue (Rendering|Material|CreateDynamicMaterialInstance (Variables|Default|GetSphere) 0 "/Game/_Project/Materials/M_Bomb.M_Bomb" :!class /Script/Engine.PrimitiveComponent))
  (Variables|Default|SetDynamicMaterial _returnvalue)
  (Variables|Default|SetBlastFxBP "/Game/_Project/Blueprints/Dynamic/BP_BlastFx.BP_BlastFx_C"))

(fn OnBlastTimeEnd
  (Class|Bomb|Detonate))