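; BP_SaveGame is a save game object that tracks match victory counts for player 1 and player 2.
; Each increment function loads the "MatchValues" slot, casts it to BP_SaveGame, increments that player's counter and saves the loaded object back to the slot.
; IncrementP2Victories also assigns the result to its own P2Victories, whereas the P1 version assigns it to the loaded object.
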(fn IncrementP1Victories
  (bind _returnvalue (SaveGame|LoadGamefromSlot "MatchValues"))
  (bind _asbp_save_game (Utilities|Casting|CastToBP_SaveGame _returnvalue))
  (bind _result (Math|Integer|IncrementInt (Variables|BP_SaveGame_C|GetP1_Victories _asbp_save_game))
    (:%20%20
      (Variables|BP_SaveGame_C|SetP1_Victories _asbp_save_game _result)
      (SaveGame|SaveGametoSlot _asbp_save_game "MatchValues"))))

(fn IncrementP2Victories
  (bind _returnvalue (SaveGame|LoadGamefromSlot "MatchValues"))
  (bind _asbp_save_game (Utilities|Casting|CastToBP_SaveGame _returnvalue))
  (bind _result (Math|Integer|IncrementInt (Variables|BP_SaveGame_C|GetP2_Victories _asbp_save_game))
    (:%20%20
      (Variables|Default|SetP2_Victories _result)
      (SaveGame|SaveGametoSlot _asbp_save_game "MatchValues"))))