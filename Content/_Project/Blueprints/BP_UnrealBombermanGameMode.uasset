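; Game mode for a local multiplayer Bomberman game that runs the match countdown and relays player deaths.
; BeginPlay starts the timer, spawns a second local player, tints its character red through a dynamic material and caches all player characters.
; Tick counts down and fires the timer-end dispatcher once at zero, while PlayerDeath rebroadcasts through its own dispatcher.
; RestartGame removes the second player and destroys its pawn.
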(event Custom|PlayerDeath
  (params (DeadPlayer :type BP%20Player%20Char%20Object%20Reference))
  (Default|CallOnPlayerDeath DeadPlayer))

(event Custom|RestartGame
  (Class|GameplayStatics|RemovePlayer (Game|GetPlayerController 1) true))

(event EventBeginPlay
  (Variables|Default|SetTimer (Variables|Default|GetGameDuration))
  (bind _returnvalue (Class|GameplayStatics|CreatePlayer 1))
  (bind _asbp_player_char (Utilities|Casting|CastToBP_PlayerChar (Pawn|GetControlledPawn _returnvalue)))
  (Rendering|Material|SetVectorParameterValue (Variables|/Game/_Project/Blueprints/BP_PlayerChar.BP_PlayerChar_C|GetDynamicMaterial _asbp_player_char) "Color" "(R=0.552083,G=0.022713,B=0.017222,A=1.000000)" :!class /Script/Engine.MaterialInstanceDynamic)
  (bind _outactors (Actor|GetAllActorsOfClass "/Game/_Project/Blueprints/BP_PlayerChar.BP_PlayerChar_C"))
  (Variables|Default|SetPlayers _outactors))

(event EventTick
  (params (DeltaSeconds :type Float%20%28single-precision%29))
  (Variables|Default|SetTimer (- (Variables|Default|GetTimer) DeltaSeconds))
  (if (<= (Variables|Default|GetTimer) 0.0)
    (Utilities|FlowControl|DoOnce false
      (:Completed
        (Default|CallOnTimerEnd)))))

(fn ConstructionScript)