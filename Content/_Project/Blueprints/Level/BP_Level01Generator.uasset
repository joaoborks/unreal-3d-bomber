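; BP_Level01Generator is the Level 01 generator, setting up and resetting the breakable block layout.
; Its construction script picks the block Blueprint, fills IgnoredPoints with fixed positions near the corners, and calls CalculatePoints.
; BeginPlay recalculates the points before running parent logic.
; OnReset destroys every breakable block in reverse order, flagging each as Resetting first, then calls SpawnBlocks.
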(event EventOnReset
  (bind _outactors (Actor|GetAllActorsOfClass "/Game/_Project/Blueprints/Dynamic/BP_BlockBreakable.BP_BlockBreakable_C"))
  (bind _arrayelement (Utilities|Array|ReverseforEachLoop _outactors)
    (:LoopBody
      (Variables|/Game/_Project/Blueprints/Dynamic/BP_BlockBreakable.BP_BlockBreakable_C|SetResetting _arrayelement true)
      (Actor|DestroyActor _arrayelement))
    (:Completed
      (Class|BlockGenerator|SpawnBlocks))))

(event EventBeginPlay
  (Class|BlockGenerator|CalculatePoints)
  (|CallParentFunction))

(fn ConstructionScript
  (bind _ignoredpoints (Variables|Default|GetIgnoredPoints))
  (Utilities|FlowControl|Sequence
    (:then_0
      (Variables|Default|SetBlockBreakableBP "/Game/_Project/Blueprints/Dynamic/BP_BlockBreakable.BP_BlockBreakable_C")
      (Utilities|Array|Clear _ignoredpoints)
      (Utilities|Array|Add _ignoredpoints "-700.000000,-700.000000,0")
      (Utilities|Array|Add _ignoredpoints "700.000000,700.000000,0")
      (Utilities|Array|Add _ignoredpoints "700.000000,600.000000,0")
      (Utilities|Array|Add _ignoredpoints "700.000000,-600.000000,0")
      (Utilities|Array|Add _ignoredpoints "-700.000000,600.000000,0")
      (Utilities|Array|Add _ignoredpoints "-700.000000,-600.000000,0")
      (Utilities|Array|Add _ignoredpoints "600.000000,700.000000,0")
      (Utilities|Array|Add _ignoredpoints "600.000000,-700.000000,0")
      (Utilities|Array|Add _ignoredpoints "-600.000000,700.000000,0")
      (Utilities|Array|Add _ignoredpoints "-600.000000,-700.000000,0"))
    (:then_1
      (Class|BlockGenerator|CalculatePoints))))