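; Player controller that turns axis and action input into movement and bomb placement for the possessed pawn.
; Vertical and Horizontal axes add movement input along the pawn's forward and right vectors whenever a valid pawn is controlled.
; Pressing Bomb casts the pawn to BP_PlayerChar and calls its SpawnBomb.
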(event Input|ActionEvents|InputActionBomb
  (params (Key :type Key%20Structure))
  (:Pressed
    (bind _asbp_player_char (Utilities|Casting|CastToBP_PlayerChar (Pawn|GetControlledPawn)))
    (Default|SpawnBomb _asbp_player_char)))

(event Input|AxisEvents|InputAxisVertical
  (params (AxisValue :type Float%20%28single-precision%29))
  (bind _returnvalue (Pawn|GetControlledPawn))
  (Utilities|IsValid _returnvalue
    (:Is%20Valid
      (Pawn|Input|AddMovementInput _returnvalue (Transformation|GetActorForwardVector _returnvalue) AxisValue false))))

(event Input|AxisEvents|InputAxisHorizontal
  (params (AxisValue :type Float%20%28single-precision%29))
  (bind _returnvalue (Pawn|GetControlledPawn))
  (Utilities|IsValid _returnvalue
    (:Is%20Valid
      (Pawn|Input|AddMovementInput _returnvalue (Transformation|GetActorRightVector _returnvalue) AxisValue false))))

(fn ConstructionScript)